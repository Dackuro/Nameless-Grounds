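; Player spawn platform with an example enemy robot that faces the player and reacts to being shot.
; Tick rotates the enemy's pitch and yaw toward the player character's EnemyAimPoint, cached on BeginPlay.
; When the player leaves SpawnArea, a short timer hides the platform and disables its collision.
; Bullets overlapping CollisionCapsule show a random taunt text, which another timer hides.
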(event `self.ReceiveBeginPlay`
  ;[1 1 1] Quickly added to make the example enemy look at the enemy.
  (bind _asbp_first_person_character_v2 (cast `/Game/Player/BP_FirstPersonCharacterV2` (`GameplayStatics.GetPlayerCharacter` 0)))
  (bind _output_get (set `self.PlayerRef` _asbp_first_person_character_v2))
  (set `self.Enemy Aim Point` (`/Game/Player/BP_FirstPersonCharacterV2.EnemyAimPoint` _output_get)))

(event `self.ReceiveTick`
  (params (DeltaSeconds :type "Float (single-precision)"))
  (bind _exampleenemy (`self.ExampleEnemy`))
  (bind (_returnvalue_roll _returnvalue_pitch _returnvalue_yaw) (`KismetMathLibrary.BreakRotator` (`KismetMathLibrary.FindLookAtRotation` (`SceneComponent.K2_GetComponentLocation` _exampleenemy) (`SceneComponent.K2_GetComponentLocation` (`self.Enemy Aim Point`)))))
  ;[1 1 1] Quickly added to make the example enemy look at the enemy.
  (`SceneComponent.K2_SetWorldRotation` _exampleenemy (`KismetMathLibrary.MakeRotator` 0.0 _returnvalue_pitch _returnvalue_yaw) false false))

(event `self.SpawnArea.OnComponentEndOverlap`
  (params (OverlappedComponent :type "PrimitiveComponent Object Reference") (OtherActor :type "Actor Object Reference") (OtherComp :type "PrimitiveComponent Object Reference") (OtherBodyIndex :type Integer))
  ;[1 1 1] "Despawn" platform when starting game. Makes it prettier to look at.
  (if (== OtherActor (`self.PlayerRef`))
    (`KismetSystemLibrary.K2_SetTimerDelegate` (delegate `HidePlatform`) 1.2)))

(event `HidePlatform`
  (bind _platform (`self.Platform`))
  ;[1 1 1] "Despawn" platform when starting game. Makes it prettier to look at.
  (`SceneComponent.SetVisibility` _platform false true)
  (`PrimitiveComponent.SetCollisionEnabled` _platform "NoCollision"))

(event `self.CollisionCapsule.OnComponentBeginOverlap`
  (params (OverlappedComponent :type "PrimitiveComponent Object Reference") (OtherActor :type "Actor Object Reference") (OtherComp :type "PrimitiveComponent Object Reference") (OtherBodyIndex :type Integer) (bFromSweep :type Boolean) (SweepResult :type "HitResult Structure (by ref)"))
  ;[1 1 1] Attack robot.
  (cast `/Game/Bullet/BP_Bullet` OtherActor)
  (`TextRenderComponent.K2_SetText` (`self.DamagedEnemy Text`) (`KismetArrayLibrary.Array_Random` (`|MakeArray` "Ouch!" "Hey!" "Watch it!" "Oof!" "That hurts!" "Bring it!" "Come on!" "More!" :!type "Text"))) ; Randomize text. Gives life to robot.
  (`SceneComponent.SetVisibility` (`self.DamagedEnemy Text`) true false)
  (`KismetSystemLibrary.K2_SetTimerDelegate` (delegate `HideText`) 1.5))

(event `HideText`
  ;[1 1 1] Attack robot.
  (`SceneComponent.SetVisibility` (`self.DamagedEnemy Text`) false false))

(fn `UserConstructionScript`)