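; BP_EnemySpawner spawns BP_Enemy at its own transform, keeping one live enemy at a time once the player has started.
; A looping timer checks the player's HasStarted and its own CanSpawnEnemy flag before each spawn.
; Each spawn fires OnEnemySpawn for the HUD and binds to the enemy's death event, which re-allows spawning after a random delay.
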(event `self.ReceiveBeginPlay`
  ;[1 1 1] Sets enemy spawn and gets reference to player.
  (`KismetSystemLibrary.K2_SetTimerDelegate` (delegate `SpawnEnemy`) 2.0 true)
  (bind _asbp_first_person_character_v2 (cast `/Game/Player/BP_FirstPersonCharacterV2` (`GameplayStatics.GetPlayerCharacter` 0)))
  (set `self.PlayerRef` _asbp_first_person_character_v2))

(event `SpawnEnemy`
  ;[1 1 1] Spawn enemy only if allowed.
  (if (and (`/Game/Player/BP_FirstPersonCharacterV2.hasStarted` (`self.PlayerRef`)) (`self.canSpawnEnemy`))
    (bind _returnvalue (`|SpawnActorFromClass` "/Game/EnemyRobot/BP_Enemy.BP_Enemy_C" (`self.GetTransform`) "AlwaysSpawn" "OverrideRootScale" null null))
    (bind _output_get (set `self.enemySpawned` _returnvalue))
    (`self.onEnemySpawn` _output_get) ; Binded from HUD.
    (add `/Game/EnemyRobot/BP_Enemy.onEnemyDeath` _output_get (delegate `SetTimerForSpawn`)) ; Repeat process if enemy dead.
    (set `self.canSpawnEnemy` false)))

(event `SetTimerForSpawn`
  ;[1 1 1] Spawn enemy only if allowed.
  (`KismetSystemLibrary.K2_SetTimerDelegate` (delegate `AllowSpawn`) (`KismetMathLibrary.RandomFloatInRange` 10.0 20.0)))

(event `AllowSpawn`
  ;[1 1 1] Spawn enemy only if allowed.
  (set `self.canSpawnEnemy` true))

(fn `UserConstructionScript`)