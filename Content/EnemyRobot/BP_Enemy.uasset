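; Robot enemy that turns its mesh toward the player's aim point every tick and fires projectiles at them.
; A forward line trace from the muzzle confirms the player is visible before spawning BP_Bullet, then a randomized timer gates the next shot.
; Health, damage and healing are delegated to DamageSystemBP.
; Death broadcasts OnEnemyDeath, plays explosion effects, hides and disables collision, then destroys the actor after a short delay.
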(event `self.ReceiveBeginPlay`
  ;[1 1 1] Get reference to player.
  (bind _asbp_first_person_character_v2 (cast `/Game/Player/BP_FirstPersonCharacterV2` (`GameplayStatics.GetPlayerCharacter` 0)))
  (set `self.aimAtLocation` (`/Game/Player/BP_FirstPersonCharacterV2.EnemyAimPoint` _asbp_first_person_character_v2)))

(event `self.ReceiveTick`
  (params (DeltaSeconds :type "Float (single-precision)"))
  ;[1 1 1] Aims at player and tries to shoot at it. Only if player is alive.
  (if (`KismetSystemLibrary.IsValid` (`self.aimAtLocation`))
    (`self.RotateToPlayer`)
    (`self.Shoot`)))

(event `Shoot`
  ;[1 1 1] Checks if can shoot at player. If allowed, shoots and goes on cooldown.
  (if (`self.canShoot`)
    (`self.AimSystem`)
    (if (`self.playerVisible`)
      (`self.ShootAtPlayer`))))

(event `ReloadCooldown`
  ;[1 1 1] Checks if can shoot at player. If allowed, shoots and goes on cooldown.
  (set `self.canShoot` true))

(event `Death`
  ;[1 1 1] Called when Killed: Adds a point to the total, sets the actor invisible and with no collision and after a brief delay, it destroys itself.
  (set `self.isDead` true) ; Used in the bullet bp.
  (`self.onEnemyDeath`)
  (`KismetSystemLibrary.K2_SetTimerDelegate` (delegate `DestroyActor`) 2.0) ; I added a delay to prevent possible problems with destruction.
  (`SceneComponent.SetVisibility` (`self.Mesh`) false false)
  (`PrimitiveComponent.SetCollisionEnabled` (`self.CapsuleComponent`) "NoCollision")
  (`PrimitiveComponent.SetCollisionEnabled` (`self.Mesh`) "NoCollision")
  (`GameplayStatics.SpawnEmitterAtLocation` "/Game/Particles/P_Explosion.P_Explosion" (`SceneComponent.K2_GetComponentLocation` (`self.Mesh`)) (struct) (0.7 0.7 0.7))
  (`AudioComponent.Play` (`self.AudioSource`) 0.0))

(event `DestroyActor`
  ;[1 1 1] Called when Killed: Adds a point to the total, sets the actor invisible and with no collision and after a brief delay, it destroys itself.
  (`self.K2_DestroyActor`))

(fn `AimSystem`
  (bind _bulletstartingpoint (`self.BulletStartingPoint`))
  (bind _returnvalue (`SceneComponent.K2_GetComponentLocation` _bulletstartingpoint))
  ;[1 1 1] Aims constantly at the player. Returns playerVisible bool.
  (bind (_outhit _returnvalue_2) (`KismetSystemLibrary.LineTraceSingle` _returnvalue (+ _returnvalue (* (`SceneComponent.GetForwardVector` _bulletstartingpoint) 50000.0)) "TraceTypeQuery5"))
  (if _returnvalue_2
    (cast `/Game/Player/BP_FirstPersonCharacterV2` (`.HitActor` (`GameplayStatics.BreakHitResult` _outhit))
      (:`then`
        (set `self.playerVisible` true))
      (:`CastFailed`
        (set `self.playerVisible` false :!label _label)))
    (else
      (goto _label))))

(fn `GetCurrentHealth`
  (returns (health :type "Float (double-precision)"))
  (return (`/Game/ActorComponents/BP_DamageSystem.health` (`self.DamageSystem_BP`))))

(fn `GetMaxHealth`
  (returns (maxHealth :type "Float (double-precision)"))
  (return (`/Game/ActorComponents/BP_DamageSystem.maxHealth` (`self.DamageSystem_BP`))))

(fn `Heal`
  (params (healAmount :type "Float (double-precision)"))
  (returns (newHealth :type "Float (double-precision)"))
  (bind _newhealth (`/Game/ActorComponents/BP_DamageSystem.Heal` (`self.DamageSystem_BP`) healAmount))
  (return _newhealth))

(fn `RotateToPlayer`
  (bind _mesh (`self.Mesh`))
  (bind (_returnvalue_roll _returnvalue_pitch _returnvalue_yaw) (`KismetMathLibrary.BreakRotator` (`KismetMathLibrary.FindLookAtRotation` (`SceneComponent.K2_GetComponentLocation` _mesh) (`SceneComponent.K2_GetComponentLocation` (`self.aimAtLocation`)))))
  ;[1 1 1] Calculates the rotation needed to look at the player and applies it.
  (`SceneComponent.K2_SetWorldRotation` _mesh (`KismetMathLibrary.MakeRotator` 0.0 _returnvalue_pitch _returnvalue_yaw) false false))

(fn `ShootAtPlayer`
  (bind (_returnvalue_location _returnvalue_rotation) (`KismetMathLibrary.BreakTransform` (`SceneComponent.K2_GetComponentToWorld` (`self.BulletStartingPoint`))))
  ;[1 1 1] Basic shooting logic. Spawns projectile and claims this BP as owner. Also adds a timer until the actor can shoot again.
  (bind _returnvalue (`|SpawnActorFromClass` "/Game/Bullet/BP_Bullet.BP_Bullet_C" (`KismetMathLibrary.MakeTransform` _returnvalue_location _returnvalue_rotation) "AlwaysSpawn" "OverrideRootScale" self "/Game/Bullet/Materials/M_EnemyEffect.M_EnemyEffect" (`self.bulletColor`) null))
  (`PrimitiveComponent.IgnoreActorWhenMoving` (`self.CapsuleComponent`) _returnvalue true)
  (`ActorComponent.Activate` (`self.BulletStartingPoint`) true)
  (set `self.canShoot` false)
  (`KismetSystemLibrary.K2_SetTimerDelegate` (`|CreateDelegate` :!event `ReloadCooldown`) (`KismetMathLibrary.RandomFloatInRange` 4.0 7.0)))

(fn `TakeDamage`
  (params (damageAmount :type "Float (double-precision)"))
  (`/Game/ActorComponents/BP_DamageSystem.TakeDamage` (`self.DamageSystem_BP`) damageAmount)
  (return))

(fn `UserConstructionScript`
  (add `/Game/ActorComponents/BP_DamageSystem.OnDeath` (`self.DamageSystem_BP`) (`|CreateDelegate` :!event `Death`))
  (`NiagaraComponent.SetVariableLinearColor` (`self.BulletStartingPoint`) "User.SetColor" (`self.bulletColor`)) ; Set shooting particle color.
)