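; BP_DamageSystem is a damage component that tracks an actor's health and death state.
; Heal adds to Health, clamps it between zero and MaxHealth, and returns the new value.
; TakeDamage subtracts from Health without clamping, then sets IsDead and calls OnDeath for death-specific events once Health reaches zero or below.
; Both functions only change Health while IsDead is false.
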(fn `Heal`
  (params (healAmount :type "Float (double-precision)"))
  (returns (newHealth :type "Float (double-precision)"))
  ;[1 1 1] Calculates HP healed.
  (if (not (`self.isDead`))
    (bind _output_get (set `self.health` (`KismetMathLibrary.FClamp` (+ healAmount (`self.health`)) 0.0 (`self.maxHealth`))))
    (return _output_get)))

(fn `TakeDamage`
  (params (damageAmount :type "Float (double-precision)"))
  ;[1 1 1] Calculates damage taken and if it kills the character.
  (if (not (`self.isDead`))
    (bind _output_get (set `self.health` (- (`self.health`) damageAmount)))
    (if (<= _output_get 0.0)
      (set `self.isDead` true)
      (`self.OnDeath`) ; Calls onDeath to trigger death-specific events.
    )
    (return)))