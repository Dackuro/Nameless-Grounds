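; BP_FOV is an actor component that widens the first-person camera's field of view as its BP_FirstPersonCharacterV2 owner moves forward.
; A looping timer started on BeginPlay blends default to target FOV using the dot product of normalized velocity and actor forward.
; The clamped result is approached with constant-rate interpolation.
; Only movement direction drives the effect, not speed magnitude, and backward movement stays at the default FOV.
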(event `self.ReceiveBeginPlay`
  ;[1 1 1] Set everything needed.
  (bind _asbp_first_person_character_v2 (cast `/Game/Player/BP_FirstPersonCharacterV2` (`self.GetOwner`)))
  (`/Engine/EditorBlueprintResources/StandardMacros.IsValid` _asbp_first_person_character_v2
    (:`Is Valid`
      (set `self.PlayerRef` _asbp_first_person_character_v2)
      (`KismetSystemLibrary.K2_SetTimerDelegate` (delegate `UpdateFOV`) (`self.updateTimerTime`) true))))

(event `UpdateFOV`
  (bind _playerref (`self.PlayerRef`))
  (bind _fovdefault (`self.FOVDefault`))
  (bind _fovtarget (`self.FOVTarget`))
  (bind _firstpersoncamera (`/Game/Player/BP_FirstPersonCharacterV2.FirstPersonCamera` _playerref))
  ;[1 1 1] Update FoV based on speed, only applied to forward vector and only when positive. Going backwards won't go under 90.
  (bind _output_get (set `self.forwardAlpha` (`KismetMathLibrary.Dot_VectorVector` (`KismetMathLibrary.Normal` (`MovementComponent.Velocity` (`Pawn.GetMovementComponent` _playerref))) (`Actor.GetActorForwardVector` _playerref))))
  (`CameraComponent.SetFieldOfView` _firstpersoncamera (`KismetMathLibrary.FInterpTo_Constant` (`CameraComponent.FieldOfView` _firstpersoncamera) (`KismetMathLibrary.FClamp` (`KismetMathLibrary.Lerp` _fovdefault _fovtarget _output_get) _fovdefault _fovtarget) (`GameplayStatics.GetWorldDeltaSeconds`) (`self.interpSpeed`))))